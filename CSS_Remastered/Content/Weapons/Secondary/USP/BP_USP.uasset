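; First-person USP secondary pistol with a toggleable silencer, exposing fire, draw, reload, alt and drop actions.
; Fire is rate-gated, plays montage and sound by silencer state, line-traces from the camera to push physics objects and attach bullet holes, and auto-reloads after the last round.
; Montage-timed delays gate CanFire, Tick mirrors HasSil to the arms AnimBP, and unsilenced shots flash the muzzle.
; Drop throws a pickup actor and destroys the weapon.
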(event EventDrop
  (params (CameraForward :type Scene%20Component%20Object%20Reference))
  (bind _returnvalue (Game|SpawnActorfromClass "/Game/Weapons/Secondary/USP/BP_USP_Pickup.BP_USP_Pickup_C" (Math|Conversions|ToTransform(Vector) (Transformation|GetWorldLocation CameraForward)) "Undefined" (Components|GetOwner) 0))
  (Physics|AddForce (Variables|/Game/Weapons/Secondary/USP/BP_USP_Pickup.BP_USP_Pickup_C|GetUSP_Pickup _returnvalue) (+ (* (Math|Vector|GetForwardVector CameraForward) 5e+04) (* (Math|Vector|GetUpVector CameraForward) 2.5e+04)) "None" true)
  (Actor|DestroyActor))

(event EventFire
  (params (Camera :type Camera%20Component%20Object%20Reference))
  (bind _returnvalue (Math|Vector|GetForwardVector Camera))
  (bind _returnvalue_2 (Transformation|GetWorldLocation Camera))
  (bind _returnvalue_3 (Transformation|GetActorLocation))
  (bind _returnvalue_4 (Math|Random|RandomFloatinRange 0.9 1.1))
  (bind _muzzleflash (Variables|Default|GetMuzzleFlash))
  (bind _arms_gun (Variables|Default|GetArms_Gun))
  (bind _firerate (Variables|Default|GetFireRate))
  (bind _firerate_2 (Variables|Default|GetFireRate))
  (bind _returnvalue_5 (Components|SkeletalMesh|GetAnimInstance _arms_gun))
  (if (Variables|Default|GetCanFire)
    (if (> (Variables|Default|GetCurrentAmmo) 0)
      (Utilities|FlowControl|DoOnce false :!label _label
        (:Completed
          (if (Variables|Default|GetHasSil)
            (if (<= (Variables|Default|GetCurrentAmmo) 1)
              (bind _returnvalue_6 (Animation|Montage|MontagePlay _returnvalue_5 "/Game/Weapons/Secondary/USP/Anims/CSSUSP_v_pist_usp_qc_skeleton_shootlast_Montage.CSSUSP_v_pist_usp_qc_skeleton_shootlast_Montage" 1.0 "Duration" 0.0 true))
              (Utilities|FlowControl|Sequence
                (:then_0
                  (Utilities|FlowControl|Delay _firerate)
                  (goto _label Reset))
                (:then_1
                  (Utilities|FlowControl|Delay (/ _returnvalue_6 1.5))
                  (CallFunction|Reload))
                (:then_2
                  (if (Variables|Default|GetHasSil) :!label _label_2
                    (Audio|PlaySoundatLocation "/Game/Weapons/Secondary/USP/Sounds/usp1.usp1" _returnvalue_3 "0, 0, 0" 1.0 _returnvalue_4 0.0 0 0 0)
                    (else
                      (Audio|PlaySoundatLocation "/Game/Weapons/Secondary/USP/Sounds/usp_unsil-1.usp_unsil-1" _returnvalue_3 "0, 0, 0" 1.0 _returnvalue_4 0.0 0 0 0)))
                  (Utilities|FlowControl|Sequence
                    (:then_0
                      (Math|Integer|DecrementInt (Variables|Default|GetCurrentAmmo)))
                    (:then_1
                      (bind (_outhit _returnvalue_7) (Collision|LineTraceByChannel _returnvalue_2 (+ _returnvalue_2 (* _returnvalue 1e+04)) "TraceTypeQuery1" false 0 "None"))
                      (if _returnvalue_7
                        (if (Physics|IsSimulatingPhysics (.HitComponent (Collision|BreakHitResult _outhit)) "None")
                          (Physics|AddForce (.HitComponent (Collision|BreakHitResult _outhit)) (* _returnvalue 3e+04) "None" true))
                        (bind _returnvalue_8 (Game|SpawnActorfromClass "/Game/Objects/Bullethole/BP_Bullethole.BP_Bullethole_C" (Math|Transform|MakeTransform (.Location (Collision|BreakHitResult _outhit)) (Math|Rotator|MakeRotfromZ (.Normal (Collision|BreakHitResult _outhit)))) "Undefined" 0 0))
                        (Transformation|AttachComponentToComponent _returnvalue_8 (.HitComponent (Collision|BreakHitResult _outhit)) "None" "KeepWorld" "KeepWorld" "KeepWorld" true)))
                    (:then_2
                      (if (not (Variables|Default|GetHasSil))
                        (Transformation|SetRelativeRotation _muzzleflash (Math|Rotator|MakeRotator 1.8e+02 0.0 (Math|Random|RandomFloatinRange 0.0 3.6e+02)) false false)
                        (Rendering|SetVisibility _muzzleflash true false)
                        (Utilities|FlowControl|Delay 0.05)
                        (Rendering|SetVisibility _muzzleflash false false))))))
              (else
                (Animation|Montage|MontagePlay _returnvalue_5 "/Game/Weapons/Secondary/USP/Anims/CSSUSP_v_pist_usp_qc_skeleton_shoot1_Montage1.CSSUSP_v_pist_usp_qc_skeleton_shoot1_Montage1" 1.0 "Duration" 0.0 true)
                (Utilities|FlowControl|Sequence
                  (:then_0
                    (Utilities|FlowControl|Delay _firerate)
                    (goto _label Reset))
                  (:then_1
                    (goto _label_2)))))
            (elif (<= (Variables|Default|GetCurrentAmmo) 1)
              (bind _returnvalue_9 (Animation|Montage|MontagePlay _returnvalue_5 "/Game/Weapons/Secondary/USP/Anims/CSSUSP_v_pist_usp_qc_skeleton_shootlast_unsil_Montage.CSSUSP_v_pist_usp_qc_skeleton_shootlast_unsil_Montage" 1.0 "Duration" 0.0 true))
              (Utilities|FlowControl|Sequence
                (:then_0
                  (Utilities|FlowControl|Delay _firerate_2)
                  (goto _label Reset))
                (:then_1
                  (goto _label_2))
                (:then_2
                  (Utilities|FlowControl|Delay (/ _returnvalue_9 1.5))
                  (CallFunction|Reload)))
              (else
                (Animation|Montage|MontagePlay _returnvalue_5 "/Game/Weapons/Secondary/USP/Anims/CSSUSP_v_pist_usp_qc_skeleton_shoot1_Montage.CSSUSP_v_pist_usp_qc_skeleton_shoot1_Montage" 1.0 "Duration" 0.0 true)
                (Utilities|FlowControl|Sequence
                  (:then_0
                    (Utilities|FlowControl|Delay _firerate_2)
                    (goto _label Reset))
                  (:then_1
                    (goto _label_2))))))))
      (else
        (Audio|PlaySoundatLocation "/Game/Weapons/Secondary/USP/Sounds/clipempty_pistol.clipempty_pistol" (Transformation|GetActorLocation) "0, 0, 0" 1.0 1.0 0.0 0 0 0)))))

(event EventDraw
  (bind _arms_gun (Variables|Default|GetArms_Gun))
  (bind _returnvalue (Components|SkeletalMesh|GetAnimInstance _arms_gun))
  (Variables|Default|SetCanFire false)
  (if (Variables|Default|GetHasSil)
    (bind _returnvalue_2 (Animation|Montage|MontagePlay _returnvalue "/Game/Weapons/Secondary/USP/Anims/CSSUSP_v_pist_usp_qc_skeleton_draw_Montage.CSSUSP_v_pist_usp_qc_skeleton_draw_Montage" 1.0 "Duration" 0.0 true))
    (Utilities|FlowControl|Delay _returnvalue_2)
    (else
      (bind _returnvalue_3 (Animation|Montage|MontagePlay _returnvalue "/Game/Weapons/Secondary/USP/Anims/CSSUSP_v_pist_usp_qc_skeleton_draw_unsil_Montage.CSSUSP_v_pist_usp_qc_skeleton_draw_unsil_Montage" 1.0 "Duration" 0.0 true))
      (Utilities|FlowControl|Delay _returnvalue_3)))
  (Variables|Default|SetCanFire true))

(event EventReload
  (bind _arms_gun (Variables|Default|GetArms_Gun))
  (bind _returnvalue (Components|SkeletalMesh|GetAnimInstance _arms_gun))
  (if (and (Variables|Default|GetCanFire) (< (Variables|Default|GetCurrentAmmo) (Variables|Default|GetMaxAmmo)))
    (Variables|Default|SetCanFire false)
    (if (Variables|Default|GetHasSil)
      (bind _returnvalue_2 (Animation|Montage|MontagePlay _returnvalue "/Game/Weapons/Secondary/USP/Anims/CSSUSP_v_pist_usp_qc_skeleton_reload_Montage.CSSUSP_v_pist_usp_qc_skeleton_reload_Montage" 1.0 "Duration" 0.0 true))
      (Utilities|FlowControl|Delay _returnvalue_2)
      (else
        (bind _returnvalue_3 (Animation|Montage|MontagePlay _returnvalue "/Game/Weapons/Secondary/USP/Anims/CSSUSP_v_pist_usp_qc_skeleton_reload_unsil_Montage.CSSUSP_v_pist_usp_qc_skeleton_reload_unsil_Montage" 1.0 "Duration" 0.0 true))
        (Utilities|FlowControl|Delay _returnvalue_3)))
    (Variables|Default|SetCurrentAmmo (Variables|Default|GetMaxAmmo))
    (Variables|Default|SetCanFire true)))

(event EventAlt
  (params (Camera :type Camera%20Component%20Object%20Reference))
  (bind _arms_gun (Variables|Default|GetArms_Gun))
  (bind _returnvalue (Components|SkeletalMesh|GetAnimInstance _arms_gun))
  (if (Variables|Default|GetCanFire)
    (Utilities|FlowControl|DoOnce false :!label _label
      (:Completed
        (Variables|Default|SetCanFire false)
        (if (Variables|Default|GetHasSil)
          (bind _returnvalue_2 (Animation|Montage|MontagePlay _returnvalue "/Game/Weapons/Secondary/USP/Anims/CSSUSP_v_pist_usp_qc_skeleton_detach_silencer_Montage.CSSUSP_v_pist_usp_qc_skeleton_detach_silencer_Montage" 1.0 "Duration" 0.0 true))
          (Utilities|FlowControl|Sequence
            (:then_0
              (Utilities|FlowControl|Delay (/ _returnvalue_2 1.5))
              (Variables|Default|SetCanFire true :!label _label_2)
              (goto _label Reset))
            (:then_1
              _))
          (else
            (bind _returnvalue_3 (Animation|Montage|MontagePlay _returnvalue "/Game/Weapons/Secondary/USP/Anims/CSSUSP_v_pist_usp_qc_skeleton_add_silencer_Montage.CSSUSP_v_pist_usp_qc_skeleton_add_silencer_Montage" 1.0 "Duration" 0.0 true))
            (Utilities|FlowControl|Sequence
              (:then_0
                (Utilities|FlowControl|Delay (/ _returnvalue_3 1.5))
                (goto _label_2))
              (:then_1
                _))))
        (Variables|Default|SetHasSil (not (Variables|Default|GetHasSil)))))))

(event EventTick
  (params (DeltaSeconds :type Float%20%28single-precision%29))
  (bind _ascss_usp_abp (Utilities|Casting|CastToCSS_USP_ABP (Components|SkeletalMesh|GetAnimInstance (Variables|Default|GetArms_Gun))))
  (Variables|/Game/Weapons/Secondary/USP/Anims/CSS_USP_ABP.CSS_USP_ABP_C|SetHasSil _ascss_usp_abp (Variables|Default|GetHasSil)))

(fn ConstructionScript
  (Variables|Default|SetCurrentAmmo (Variables|Default|GetMaxAmmo)))

(fn DoesReplaceWeapon
  (return true))

(fn GetAmmo
  (return (Variables|Default|GetCurrentAmmo)))

(fn GetType
  (return "NewEnumerator1"))

(fn GetWeaponPic
  (return "/Game/Weapons/Secondary/USP/Textures/usp45.usp45"))