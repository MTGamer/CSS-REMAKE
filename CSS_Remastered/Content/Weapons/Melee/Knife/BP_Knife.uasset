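; BP_Knife is a melee weapon with Fire (slash), Alt (stab) and Draw events, reporting zero ammo.
; Fire plays a random slash montage, rate-limited by a DoOnce and delay, with a short camera trace selecting physics-hit, wall-hit or whiff sounds.
; Alt traces likewise, playing a stab montage with delayed force on physics objects, otherwise a miss montage.
; Draw and Alt lock CanFire for their montage durations; no damage is applied.
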(event EventFire
  (params (Camera :type Camera%20Component%20Object%20Reference))
  (bind _returnvalue (Transformation|GetActorLocation))
  (bind _returnvalue_2 (Transformation|GetWorldLocation Camera))
  (bind _array (Utilities|Array|MakeArray "/Game/Weapons/Melee/Knife/Sounds/knife_hit1.knife_hit1" "/Game/Weapons/Melee/Knife/Sounds/knife_hit2.knife_hit2" "/Game/Weapons/Melee/Knife/Sounds/knife_hit3.knife_hit3" "/Game/Weapons/Melee/Knife/Sounds/knife_hit4.knife_hit4"))
  (bind _array_2 (Utilities|Array|MakeArray "/Game/Weapons/Melee/Knife/Sounds/knife_slash1.knife_slash1" "/Game/Weapons/Melee/Knife/Sounds/knife_slash2.knife_slash2"))
  (bind _arms_knife (Variables|Default|GetArms_Knife))
  (bind _returnvalue_3 (Components|SkeletalMesh|GetAnimInstance _arms_knife))
  (if (Variables|Default|GetCanFire)
    (Utilities|FlowControl|DoOnce false :!label _label
      (:Completed
        (if (Math|Random|RandomBool)
          (Animation|Montage|MontagePlay _returnvalue_3 "/Game/Weapons/Melee/Knife/Anims/Knife_Anim_v_knife_t_qc_skeleton_midslash1_Montage.Knife_Anim_v_knife_t_qc_skeleton_midslash1_Montage" 1.0 "Duration" 0.0 true)
          (else
            (Animation|Montage|MontagePlay _returnvalue_3 "/Game/Weapons/Melee/Knife/Anims/Knife_Anim_v_knife_t_qc_skeleton_midslash2_Montage.Knife_Anim_v_knife_t_qc_skeleton_midslash2_Montage" 1.0 "Duration" 0.0 true)))
        (Utilities|FlowControl|Sequence
          (:then_0
            (Utilities|FlowControl|Delay (Variables|Default|GetFireRate))
            (goto _label Reset))
          (:then_1
            (bind (_outhit _returnvalue_4) (Collision|LineTraceByChannel _returnvalue_2 (+ (* (Math|Vector|GetForwardVector Camera) 1e+02) _returnvalue_2) "TraceTypeQuery1" false 0 "None"))
            (if _returnvalue_4
              (Audio|PlaySoundatLocation (select (Physics|IsSimulatingPhysics (.HitComponent (Collision|BreakHitResult _outhit)) "None") (Utilities|Array|Get(acopy) _array (Math|Random|RandomIntegerinRange 0 (Utilities|Array|Length _array))) "/Game/Weapons/Melee/Knife/Sounds/knife_hitwall1.knife_hitwall1") _returnvalue "0, 0, 0" 1.0 1.0 0.0 0 0 0)
              (if (Physics|IsSimulatingPhysics (.HitComponent (Collision|BreakHitResult _outhit)) "None")
                _)
              (else
                (Audio|PlaySoundatLocation (Utilities|Array|Get(acopy) _array_2 (Math|Random|RandomIntegerinRange 0 (Utilities|Array|Length _array_2))) _returnvalue "0, 0, 0" 1.0 1.0 0.0 0 0 0)))))))))

(event EventDraw
  (Variables|Default|SetCanFire false)
  (bind _returnvalue (Animation|Montage|MontagePlay (Components|SkeletalMesh|GetAnimInstance (Variables|Default|GetArms_Knife)) "/Game/Weapons/Melee/Knife/Anims/Knife_Anim_v_knife_t_qc_skeleton_draw_Montage.Knife_Anim_v_knife_t_qc_skeleton_draw_Montage" 1.0 "Duration" 0.0 true))
  (Utilities|FlowControl|Delay _returnvalue)
  (Variables|Default|SetCanFire true))

(event EventAlt
  (params (Camera :type Camera%20Component%20Object%20Reference))
  (bind _returnvalue (Transformation|GetWorldLocation Camera))
  (bind _returnvalue_2 (Math|Vector|GetForwardVector Camera))
  (bind _arms_knife (Variables|Default|GetArms_Knife))
  (bind _returnvalue_3 (Components|SkeletalMesh|GetAnimInstance _arms_knife))
  (if (Variables|Default|GetCanFire)
    (Variables|Default|SetCanFire false)
    (bind (_outhit _returnvalue_4) (Collision|LineTraceByChannel _returnvalue (+ (* _returnvalue_2 1e+02) _returnvalue) "TraceTypeQuery1" false 0 "None"))
    (if _returnvalue_4
      (if (Physics|IsSimulatingPhysics (.HitComponent (Collision|BreakHitResult _outhit)) "None")
        (Utilities|FlowControl|Sequence
          (:then_0
            (bind _returnvalue_5 (Animation|Montage|MontagePlay _returnvalue_3 "/Game/Weapons/Melee/Knife/Anims/Knife_Anim_v_knife_t_qc_skeleton_stab_Montage.Knife_Anim_v_knife_t_qc_skeleton_stab_Montage" 1.0 "Duration" 0.0 true))
            (Utilities|FlowControl|Delay _returnvalue_5)
            (Variables|Default|SetCanFire true :!label _label))
          (:then_1
            (Utilities|FlowControl|Delay 0.45)
            (Physics|AddForce (.HitComponent (Collision|BreakHitResult _outhit)) (* _returnvalue_2 1e+05) "None" true)))
        (else
          (bind _returnvalue_6 (Animation|Montage|MontagePlay _returnvalue_3 "/Game/Weapons/Melee/Knife/Anims/Knife_Anim_v_knife_t_qc_skeleton_stab_miss_Montage.Knife_Anim_v_knife_t_qc_skeleton_stab_miss_Montage" 1.0 "Duration" 0.0 true :!label _label_2))
          (Utilities|FlowControl|Delay _returnvalue_6)
          (goto _label)))
      (else
        (goto _label_2)))))

(fn ConstructionScript)

(fn GetAmmo
  (return 0))

(fn GetType
  (return "NewEnumerator2"))