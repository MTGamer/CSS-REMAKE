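; AK47 primary weapon actor with automatic fire, draw, reload, drop, and getters for ammo, type, picture and replacement.
; Fire and LetgoFire toggle a Tick gate, with a DoOnce and FireRate delay pacing shots.
; Each shot line traces from the supplied camera, pushes physics objects, attaches a bullet hole, and plays montage, sound and muzzle flash.
; Draw and reload montages block firing; Drop launches a pickup and destroys the weapon.
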(event EventDrop
  (params (CameraForward :type Scene%20Component%20Object%20Reference))
  (bind _returnvalue (Game|SpawnActorfromClass "/Game/Weapons/Primary/AK47/BP_AK47_Pickup.BP_AK47_Pickup_C" (Math|Conversions|ToTransform(Vector) (Transformation|GetWorldLocation CameraForward)) "Undefined" (Components|GetOwner) 0))
  (Physics|AddForce (Variables|/Game/Weapons/Primary/AK47/BP_AK47_Pickup.BP_AK47_Pickup_C|GetAK47_Pickup _returnvalue) (+ (* (Math|Vector|GetForwardVector CameraForward) 5e+04) (* (Math|Vector|GetUpVector CameraForward) 2.5e+04)) "None" true)
  (Actor|DestroyActor))

(event EventFire
  (params (Camera :type Camera%20Component%20Object%20Reference))
  (bind _muzzlefash (Variables|Default|GetMuzzleFash))
  (Variables|Default|SetCam Camera)
  (Utilities|FlowControl|Gate true) ; enters at Open
)

(event EventTick
  (params (DeltaSeconds :type Float%20%28single-precision%29))
  (bind _muzzlefash (Variables|Default|GetMuzzleFash))
  (bind _cam (Variables|Default|GetCam))
  (bind _returnvalue (Transformation|GetWorldLocation _cam))
  (bind _returnvalue_2 (Math|Vector|GetForwardVector _cam))
  (Utilities|FlowControl|Gate true
    (:Exit
      (if (Variables|Default|GetCanFire)
        (if (> (Variables|Default|GetCurrentAmmo) 0)
          (Utilities|FlowControl|DoOnce false :!label _label
            (:Completed
              (Animation|Montage|MontagePlay (Components|SkeletalMesh|GetAnimInstance (Variables|Default|GetArms_Gun)) "/Game/Weapons/Primary/AK47/Models/View/AK47_Anim_v_rif_ak47_qc_skeleton_ak47_fire1_Montage.AK47_Anim_v_rif_ak47_qc_skeleton_ak47_fire1_Montage" 1.0 "Duration" 0.0 true)
              (Utilities|FlowControl|Sequence
                (:then_0
                  (Utilities|FlowControl|Delay (Variables|Default|GetFireRate))
                  (goto _label Reset))
                (:then_1
                  (Audio|PlaySoundatLocation "/Game/Weapons/Primary/AK47/Sounds/ak47-1.ak47-1" (Transformation|GetActorLocation) "0, 0, 0" 0.5 (Math|Random|RandomFloatinRange 0.9 1.1) 0.0 0 0 0))
                (:then_2
                  (Math|Integer|DecrementInt (Variables|Default|GetCurrentAmmo)))
                (:then_3
                  (bind (_outhit _returnvalue_3) (Collision|LineTraceByChannel _returnvalue (+ _returnvalue (* _returnvalue_2 1e+04)) "TraceTypeQuery1" false 0 "None"))
                  (if _returnvalue_3
                    (if (Physics|IsSimulatingPhysics (.HitComponent (Collision|BreakHitResult _outhit)) "None")
                      (Physics|AddForce (.HitComponent (Collision|BreakHitResult _outhit)) (* _returnvalue_2 6e+04) "None" true))
                    (bind _returnvalue_4 (Game|SpawnActorfromClass "/Game/Objects/Bullethole/BP_Bullethole.BP_Bullethole_C" (Math|Transform|MakeTransform (.Location (Collision|BreakHitResult _outhit)) (Math|Rotator|MakeRotfromZ (.Normal (Collision|BreakHitResult _outhit)))) "Undefined" 0 0))
                    (Transformation|AttachComponentToComponent _returnvalue_4 (.HitComponent (Collision|BreakHitResult _outhit)) "None" "KeepWorld" "KeepWorld" "KeepWorld" true)))
                (:then_4
                  (Transformation|SetRelativeRotation _muzzlefash (Math|Rotator|MakeRotator 1.8e+02 0.0 (Math|Random|RandomFloatinRange 0.0 3.6e+02)) false false)
                  (Rendering|SetVisibility _muzzlefash true false)
                  (Utilities|FlowControl|Delay 0.05)
                  (Rendering|SetVisibility _muzzlefash false false)))))
          (else
            (Utilities|FlowControl|DoOnce false
              (:Completed
                (Audio|PlaySoundatLocation "/Game/Weapons/Primary/AK47/Sounds/clipempty_rifle.clipempty_rifle" (Transformation|GetActorLocation) "0, 0, 0" 1.0 1.0 0.0 0 0 0)))))))))

(event EventLetgoFire
  (bind _muzzlefash (Variables|Default|GetMuzzleFash))
  (Utilities|FlowControl|Sequence
    (:then_0
      (Utilities|FlowControl|DoOnce false) ; enters at Reset
    )
    (:then_1
      (Variables|Default|SetCam 0)
      (Utilities|FlowControl|Gate true) ; enters at Close
    )))

(event EventDraw
  (Variables|Default|SetCanFire false)
  (bind _returnvalue (Animation|Montage|MontagePlay (Components|SkeletalMesh|GetAnimInstance (Variables|Default|GetArms_Gun)) "/Game/Weapons/Primary/AK47/Models/View/AK47_Anim_v_rif_ak47_qc_skeleton_ak47_draw_Montage.AK47_Anim_v_rif_ak47_qc_skeleton_ak47_draw_Montage" 1.0 "Duration" 0.0 true))
  (Utilities|FlowControl|Delay _returnvalue)
  (Variables|Default|SetCanFire true))

(event EventReload
  (if (and (Variables|Default|GetCanFire) (< (Variables|Default|GetCurrentAmmo) (Variables|Default|GetMaxAmmo)))
    (Variables|Default|SetCanFire false)
    (bind _returnvalue (Animation|Montage|MontagePlay (Components|SkeletalMesh|GetAnimInstance (Variables|Default|GetArms_Gun)) "/Game/Weapons/Primary/AK47/Models/View/AK47_Anim_v_rif_ak47_qc_skeleton_ak47_reload_Montage.AK47_Anim_v_rif_ak47_qc_skeleton_ak47_reload_Montage" 1.0 "Duration" 0.0 true))
    (Utilities|FlowControl|Delay _returnvalue)
    (Variables|Default|SetCanFire true)
    (Variables|Default|SetCurrentAmmo (Variables|Default|GetMaxAmmo))))

(fn ConstructionScript
  (Variables|Default|SetCurrentAmmo (Variables|Default|GetMaxAmmo)))

(fn DoesReplaceWeapon
  (return true))

(fn GetAmmo
  (return (Variables|Default|GetCurrentAmmo)))

(fn GetType
  (return "NewEnumerator0"))

(fn GetWeaponPic
  (return "/Game/Weapons/Primary/AK47/Textures/ak47.ak47"))