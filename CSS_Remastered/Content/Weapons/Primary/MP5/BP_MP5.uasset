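; MP5 submachine gun weapon actor with automatic hitscan fire, ammo, draw, reload and drop.
; Fire opens a gate driven by Tick, and a DoOnce reset after FireRate paces shots until LetgoFire closes it.
; Each shot line-traces from the camera, pushes physics objects, attaches bullet holes and plays sound, montage and muzzle flash.
; Draw and reload block firing for their montage length, while Drop throws a pickup and destroys the weapon.
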(event EventDrop
  (params (CameraForward :type Scene%20Component%20Object%20Reference))
  (bind _returnvalue (Game|SpawnActorfromClass "/Game/Weapons/Primary/MP5/BP_MP5_Pickup.BP_MP5_Pickup_C" (Math|Conversions|ToTransform(Vector) (Transformation|GetWorldLocation CameraForward)) "Undefined" (Components|GetOwner) 0))
  (Physics|AddForce (Variables|/Game/Weapons/Primary/MP5/BP_MP5_Pickup.BP_MP5_Pickup_C|GetMP5_Pickup _returnvalue) (+ (* (Math|Vector|GetForwardVector CameraForward) 5e+04) (* (Math|Vector|GetUpVector CameraForward) 2.5e+04)) "None" true)
  (Actor|DestroyActor))

(event EventDraw
  (Variables|Default|SetCanFire false)
  (bind _returnvalue (Animation|Montage|MontagePlay (Components|SkeletalMesh|GetAnimInstance (Variables|Default|GetMP5)) "/Game/Weapons/Primary/MP5/Models/View/MP5_Anim_v_smg_mp5_qc_skeleton_draw_Montage.MP5_Anim_v_smg_mp5_qc_skeleton_draw_Montage" 1.0 "MontageLength" 0.0 true))
  (Utilities|FlowControl|Delay _returnvalue)
  (Variables|Default|SetCanFire true))

(event EventFire
  (params (Camera :type Camera%20Component%20Object%20Reference))
  (bind _muzzleflash (Variables|Default|GetMuzzleFlash))
  (Variables|Default|SetCamera Camera)
  (Utilities|FlowControl|Gate true) ; enters at Open
)

(event EventTick
  (params (DeltaSeconds :type Float%20%28single-precision%29))
  (bind _muzzleflash (Variables|Default|GetMuzzleFlash))
  (bind _camera (Variables|Default|GetCamera))
  (bind _returnvalue (Transformation|GetWorldLocation _camera))
  (bind _returnvalue_2 (Math|Vector|GetForwardVector _camera))
  (Utilities|FlowControl|Gate true
    (:Exit
      (if (and (Variables|Default|GetCanFire) (> (Variables|Default|GetAmmo) 0))
        (Utilities|FlowControl|DoOnce false :!label _label
          (:Completed
            (Utilities|FlowControl|Sequence
              (:then_0
                (Math|Integer|DecrementInt (Variables|Default|GetAmmo)
                  (:%20%20
                    (bind (_outhit _returnvalue_3) (Collision|LineTraceByChannel _returnvalue (+ _returnvalue (* _returnvalue_2 1e+04)) "TraceTypeQuery1" false 0 "None"))
                    (if _returnvalue_3
                      (if (Physics|IsSimulatingPhysics (.HitComponent (Collision|BreakHitResult _outhit)) "None")
                        (Physics|AddForce (.HitComponent (Collision|BreakHitResult _outhit)) (* _returnvalue_2 3e+04) "None" true))
                      (bind _returnvalue_4 (Game|SpawnActorfromClass "/Game/Objects/Bullethole/BP_Bullethole.BP_Bullethole_C" (Math|Transform|MakeTransform (.Location (Collision|BreakHitResult _outhit)) (Math|Rotator|MakeRotfromZ (.Normal (Collision|BreakHitResult _outhit)))) "Undefined" 0 0))
                      (Transformation|AttachComponentToComponent _returnvalue_4 (.HitComponent (Collision|BreakHitResult _outhit)) "None" "KeepWorld" "KeepWorld" "KeepWorld" true)))))
              (:then_1
                (Audio|PlaySoundatLocation "/Game/Weapons/Primary/MP5/Sounds/mp5-1.mp5-1" (Transformation|GetActorLocation) "0, 0, 0" 1.0 1.0 0.0 0 0 0)
                (Animation|Montage|MontagePlay (Components|SkeletalMesh|GetAnimInstance (Variables|Default|GetMP5)) "/Game/Weapons/Primary/MP5/Models/View/MP5_Anim_v_smg_mp5_qc_skeleton_shoot1_Montage.MP5_Anim_v_smg_mp5_qc_skeleton_shoot1_Montage" 1.0 "MontageLength" 0.0 true)
                (Utilities|FlowControl|Delay (Variables|Default|GetFireRate))
                (goto _label Reset))
              (:then_2
                (Transformation|SetRelativeRotation _muzzleflash (Math|Rotator|MakeRotator -90.000137 (Math|Random|RandomFloatinRange 0.0 3.6e+02) 0.0) false false)
                (Rendering|SetVisibility _muzzleflash true false)
                (Utilities|FlowControl|Delay 0.05)
                (Rendering|SetVisibility _muzzleflash false false)))))))))

(event EventLetgoFire
  (bind _muzzleflash (Variables|Default|GetMuzzleFlash))
  (Variables|Default|SetCamera 0)
  (Utilities|FlowControl|Gate true) ; enters at Close
)

(event EventReload
  (if (and (Variables|Default|GetCanFire) (< (Variables|Default|GetAmmo) (Variables|Default|GetMaxAmmo)))
    (Variables|Default|SetCanFire false)
    (bind _returnvalue (Animation|Montage|MontagePlay (Components|SkeletalMesh|GetAnimInstance (Variables|Default|GetMP5)) "/Game/Weapons/Primary/MP5/Models/View/MP5_Anim_v_smg_mp5_qc_skeleton_reload1_Montage.MP5_Anim_v_smg_mp5_qc_skeleton_reload1_Montage" 1.0 "MontageLength" 0.0 true))
    (Utilities|FlowControl|Delay _returnvalue)
    (Variables|Default|SetAmmo (Variables|Default|GetMaxAmmo))
    (Variables|Default|SetCanFire true)))

(fn ConstructionScript
  (Variables|Default|SetAmmo (Variables|Default|GetMaxAmmo)))

(fn DoesReplaceWeapon
  (return true))

(fn GetAmmo
  (return (Variables|Default|GetAmmo)))

(fn GetType
  (return "NewEnumerator0"))

(fn GetWeaponPic
  (return "/Game/Weapons/Primary/MP5/Textures/mp5.mp5"))