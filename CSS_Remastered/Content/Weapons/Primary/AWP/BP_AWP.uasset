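; AWP sniper rifle weapon actor with a toggleable scope, reload, droppable pickup and getters for ammo, type and picture.
; Alt toggles camera FOV zoom and a scope widget, which firing and reloading remove.
; Fire line-traces from the camera, pushing physics objects and attaching bullet holes, with an empty click when out of ammo.
; Montage lengths time the draw and reload locks and the DoOnce gate between shots.
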(event Custom|Remove%20Scope
  (bind _savedcam (Variables|Default|GetSavedCam))
  (Utilities|IsValid (Variables|Default|GetScopeUI)
    (:Is%20Valid
      (Widget|RemovefromParent (Variables|Default|GetScopeUI))
      (Variables|Default|SetScopeUI 0)
      (Utilities|IsValid _savedcam
        (:Is%20Valid
          (Camera|SetFieldOfView _savedcam 9e+01))
        (:Is%20Not%20Valid
          _))
      (Variables|Default|SetIsScoped false))))

(event EventDrop
  (params (CameraForward :type Scene%20Component%20Object%20Reference))
  (bind _returnvalue (Game|SpawnActorfromClass "/Game/Weapons/Primary/AWP/BP_AWP_Pickup.BP_AWP_Pickup_C" (Math|Conversions|ToTransform(Vector) (Transformation|GetWorldLocation CameraForward)) "Undefined" (Components|GetOwner) 0))
  (Physics|AddForce (Variables|/Game/Weapons/Primary/AWP/BP_AWP_Pickup.BP_AWP_Pickup_C|GetAWP_Pickup _returnvalue) (+ (* (Math|Vector|GetForwardVector CameraForward) 5e+04) (* (Math|Vector|GetUpVector CameraForward) 2.5e+04)) "None" true)
  (Actor|DestroyActor))

(event EventDraw
  (Variables|Default|SetCanFire false)
  (bind _returnvalue (Animation|Montage|MontagePlay (Components|SkeletalMesh|GetAnimInstance (Variables|Default|GetAWP)) "/Game/Weapons/Primary/AWP/Models/View/AWP_Anim_v_snip_awp_qc_skeleton_awm_draw_Montage.AWP_Anim_v_snip_awp_qc_skeleton_awm_draw_Montage" 1.0 "MontageLength" 0.0 true))
  (Utilities|FlowControl|Delay _returnvalue)
  (Variables|Default|SetCanFire true))

(event EventFire
  (params (Camera :type Camera%20Component%20Object%20Reference))
  (bind _returnvalue (Transformation|GetWorldLocation Camera))
  (bind _returnvalue_2 (Math|Vector|GetForwardVector Camera))
  (bind _returnvalue_3 (Transformation|GetActorLocation))
  (if (Variables|Default|GetCanFire)
    (if (> (Variables|Default|GetAmmo) 0)
      (Utilities|FlowControl|DoOnce false :!label _label
        (:Completed
          (Math|Integer|DecrementInt (Variables|Default|GetAmmo)
            (:%20%20
              (Audio|PlaySoundatLocation "/Game/Weapons/Primary/AWP/Sounds/awp1.awp1" _returnvalue_3 "0, 0, 0" 1.0 1.0 0.0 0 0 0)
              (bind _returnvalue_4 (Animation|Montage|MontagePlay (Components|SkeletalMesh|GetAnimInstance (Variables|Default|GetAWP)) "/Game/Weapons/Primary/AWP/Models/View/AWP_Anim_v_snip_awp_qc_skeleton_awm_fire_Montage.AWP_Anim_v_snip_awp_qc_skeleton_awm_fire_Montage" 1.0 "MontageLength" 0.0 true))
              (Camera|SetFieldOfView Camera 9e+01)
              (CallFunction|RemoveScope)
              (Utilities|FlowControl|Sequence
                (:then_0
                  (Utilities|FlowControl|Delay _returnvalue_4)
                  (goto _label Reset))
                (:then_1
                  (bind (_outhit _returnvalue_5) (Collision|LineTraceByChannel _returnvalue (+ (* _returnvalue_2 1e+04) _returnvalue) "TraceTypeQuery1" false 0 "None"))
                  (if _returnvalue_5
                    (if (Physics|IsSimulatingPhysics (.HitComponent (Collision|BreakHitResult _outhit)) "None")
                      (Physics|AddForce (.HitComponent (Collision|BreakHitResult _outhit)) (* _returnvalue_2 6e+04) "None" true))
                    (bind _returnvalue_6 (Game|SpawnActorfromClass "/Game/Objects/Bullethole/BP_Bullethole.BP_Bullethole_C" (Math|Transform|MakeTransform (.Location (Collision|BreakHitResult _outhit)) (Math|Rotator|MakeRotfromZ (.Normal (Collision|BreakHitResult _outhit)))) "Undefined" 0 0))
                    (Transformation|AttachComponentToComponent _returnvalue_6 (.HitComponent (Collision|BreakHitResult _outhit)) "None" "KeepWorld" "KeepWorld" "KeepWorld" true))))))))
      (else
        (Utilities|FlowControl|DoOnce false
          (:Completed
            (Audio|PlaySoundatLocation "/Game/Weapons/Primary/AK47/Sounds/clipempty_rifle.clipempty_rifle" _returnvalue_3 "0, 0, 0" 1.0 1.0 0.0 0 0 0)))))))

(event EventLetgoFire
  (Utilities|FlowControl|DoOnce false) ; enters at Reset
)

(event EventReload
  (if (and (Variables|Default|GetCanFire) (< (Variables|Default|GetAmmo) (Variables|Default|GetMaxAmmo)))
    (CallFunction|RemoveScope)
    (Variables|Default|SetCanFire false)
    (bind _returnvalue (Animation|Montage|MontagePlay (Components|SkeletalMesh|GetAnimInstance (Variables|Default|GetAWP)) "/Game/Weapons/Primary/AWP/Models/View/AWP_Anim_v_snip_awp_qc_skeleton_awm_reload_Montage.AWP_Anim_v_snip_awp_qc_skeleton_awm_reload_Montage" 1.0 "MontageLength" 0.0 true))
    (Utilities|FlowControl|Delay _returnvalue)
    (Variables|Default|SetAmmo (Variables|Default|GetMaxAmmo))
    (Variables|Default|SetCanFire true)))

(event EventAlt
  (params (Camera :type Camera%20Component%20Object%20Reference))
  (if (Variables|Default|GetCanFire)
    (Audio|PlaySoundatLocation "/Game/Weapons/Primary/AWP/Sounds/zoom.zoom" (Transformation|GetActorLocation) "0, 0, 0" 1.0 1.0 0.0 0 0 0)
    (if (Variables|Default|GetIsScoped)
      (Variables|Default|SetSavedCam 0)
      (Camera|SetFieldOfView Camera 9e+01)
      (CallFunction|RemoveScope)
      (else
        (Variables|Default|SetSavedCam Camera)
        (Camera|SetFieldOfView Camera 2e+01)
        (bind _returnvalue (UserInterface|CreateWidget "/Game/Weapons/Primary/AWP/Blueprints/Scope_UI.Scope_UI_C" (Game|GetPlayerController 0)))
        (bind _output_get (Variables|Default|SetScopeUI _returnvalue))
        (UserInterface|Viewport|AddtoViewport _output_get 0)))
    (Variables|Default|SetIsScoped (not (Variables|Default|GetIsScoped)))))

(fn ConstructionScript
  (Variables|Default|SetAmmo (Variables|Default|GetMaxAmmo)))

(fn DoesReplaceWeapon
  (return true))

(fn GetAmmo
  (return (Variables|Default|GetAmmo)))

(fn GetType
  (return "NewEnumerator0"))

(fn GetWeaponPic
  (return "/Game/Weapons/Primary/AWP/Textures/awp.awp"))