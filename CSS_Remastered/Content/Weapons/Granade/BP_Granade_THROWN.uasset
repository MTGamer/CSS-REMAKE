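; Thrown grenade actor that explodes five seconds after spawning, with sound and a scaled particle effect.
; A multi-sphere trace finds nearby objects and sends distance-tiered damage through HealthInterface, using DamagedActors to hit each actor once.
; Physics-simulating hits receive a fixed-vector impulse and trigger camera shake, and the grenade destroys itself if the trace hit anything.
; While moving, overlaps on HitColl play a bounce sound with speed-scaled volume.
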(event OnComponentBeginOverlap(HitColl)
  (params (OverlappedComponent :type Primitive%20Component%20Object%20Reference) (OtherActor :type Actor%20Object%20Reference) (OtherComp :type Primitive%20Component%20Object%20Reference) (OtherBodyIndex :type Integer) (bFromSweep :type Boolean) (SweepResult :type Hit%20Result%20Structure%20%28by%20ref%29))
  (bind _granade_world_thrown (Variables|Default|GetGranade_World_THROWN))
  (bind _returnvalue (Transformation|GetComponentVelocity _granade_world_thrown))
  (bind _returnvalue_2 (Math|Vector|VectorLength _returnvalue))
  (if (> _returnvalue_2 5.0)
    (Audio|PlaySoundatLocation "/Game/Weapons/Granade/Sounds/he_bounce-1.he_bounce-1" (Transformation|GetActorLocation) "0, 0, 0" (/ _returnvalue_2 5e+02) 1.0 0.0 0 0 0)))

(event EventBeginPlay
  (bind _granade_world_thrown (Variables|Default|GetGranade_World_THROWN))
  (bind _granade_world_thrown_2 (Variables|Default|GetGranade_World_THROWN))
  (bind _returnvalue (Transformation|GetWorldLocation _granade_world_thrown))
  (bind _returnvalue_2 (Transformation|GetWorldLocation _granade_world_thrown_2))
  (Utilities|FlowControl|Delay 5.0)
  (Audio|PlaySoundatLocation "/Game/Weapons/Granade/Sounds/explode3.explode3" _returnvalue "0, 0, 0" 1.0 1.0 0.0 "/Game/Audio/3DSOUND.3DSOUND" 0 0)
  (Utilities|FlowControl|Sequence
    (:then_0
      (Effects|SpawnEmitteratLocation "/Game/Particles/PS_GranadeExplode.PS_GranadeExplode" _returnvalue "0, 0, 0" "10.000000,10.000000,10.000000"))
    (:then_1
      (bind (_outhits _returnvalue_3) (Collision|MultiSphereTraceForObjects _returnvalue _returnvalue 5e+02 (Utilities|Array|MakeArray "ObjectTypeQuery3" "ObjectTypeQuery4" "ObjectTypeQuery2" "ObjectTypeQuery1") false 0 "None"))
      (if _returnvalue_3
        (for _array_element _outhits
          (Utilities|FlowControl|Sequence
            (:then_0
              (if (Utilities|DoesObjectImplementInterface (.HitActor (Collision|BreakHitResult _array_element)) "/Game/Blueprints/Interfaces/HealthInterface.HealthInterface_C")
                (Variables|Default|SetCanDamage true)
                (for _array_element_2 (Variables|Default|GetDamagedActors)
                  (if (== _array_element_2 (.HitActor (Collision|BreakHitResult _array_element)))
                    (Variables|Default|SetCanDamage false)))
                (if (Variables|Default|GetCanDamage)
                  (CallFunction|GranadeDamage (Math|Vector|VectorLength (- _returnvalue_2 (.ImpactPoint (Collision|BreakHitResult _array_element)))) (.HitActor (Collision|BreakHitResult _array_element)))
                  (Utilities|Array|Add (Variables|Default|GetDamagedActors) (.HitActor (Collision|BreakHitResult _array_element))))))
            (:then_1
              (if (Physics|IsSimulatingPhysics (.HitComponent (Collision|BreakHitResult _array_element)) "None")
                (Physics|AddImpulseatLocation (.HitComponent (Collision|BreakHitResult _array_element)) "6000.000000,6000.000000,6000.000000" _returnvalue_2 "None")
                (Camera|PlayWorldCameraShake "/Game/Player/Blueprints/CameraShakes/CS_Explosion.CS_Explosion_C" (Transformation|GetWorldLocation (Variables|Default|GetGranade_World_THROWN)) 8e+02 1e+03)))))
        (Actor|DestroyActor)))))

(fn ConstructionScript)

(fn GranadeDamage
  (params (Distance :type Float%20%28single-precision%29) (Damaged%20Actor :type Actor%20Object%20Reference))
  (if (<= Distance 1.2e+02)
    (LocalVariables|SetDamagedAmount 1e+02)
    (elif (<= Distance 5e+02)
      (LocalVariables|SetDamagedAmount 5e+01)
      (elif (<= Distance 1e+03)
        (LocalVariables|SetDamagedAmount 25.0)
        (else
          (LocalVariables|SetDamagedAmount 1e+01)))))
  (Class|HealthInterface|Damage(Message) Damaged%20Actor (Math|Float|Truncate (LocalVariables|GetDamagedAmount)))
  (return (Math|Float|Truncate (LocalVariables|GetDamagedAmount))))