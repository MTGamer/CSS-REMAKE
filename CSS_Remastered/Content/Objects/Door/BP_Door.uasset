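; BP_Door is a usable hinged door that toggles open and closed with metal gate sounds.
; Its Use event plays the DoorRot timeline forward or in reverse based on IsOpen, rotating the Hinge's yaw.
; A DoOnce blocks repeated use until the timeline finishes, which flips IsOpen, plays the end sound and resets the gate.
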(event EventBeginPlay)

(event EventUse
  (bind _returnvalue (Transformation|GetActorLocation))
  (Utilities|FlowControl|DoOnce false :!label _label
    (:Completed
      (if (Variables|Default|GetIsOpen)
        (Audio|PlaySoundatLocation "/Game/Objects/Door/Sounds/door_metal_gate_move1.door_metal_gate_move1" _returnvalue "0, 0, 0" 1.0 1.0 0.0 0 0 0)
        (bind _rotationz (Timeline|DoorRot Reverse)
          (:Update
            (Transformation|SetRelativeRotation (Variables|Default|GetHinge) (Math|Rotator|MakeRotator 0.0 0.0 _rotationz) false false))
          (:Finished
            (Variables|Default|SetIsOpen (not (Variables|Default|GetIsOpen)))
            (Audio|PlaySoundatLocation "/Game/Objects/Door/Sounds/door_metal_gate_close1.door_metal_gate_close1" _returnvalue "0, 0, 0" 1.0 1.0 0.0 0 0 0)
            (goto _label Reset)))
        (else
          (Audio|PlaySoundatLocation "/Game/Objects/Door/Sounds/door_metal_gate_move1.door_metal_gate_move1" _returnvalue "0, 0, 0" 1.0 1.0 0.0 0 0 0)
          (Timeline|DoorRot PlayFromStart))))))

(fn ConstructionScript)