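; Bullet hole actor that plays a surface-dependent impact sound when spawned and destroys itself after five seconds.
; On BeginPlay, a very short Visibility line trace along the Dir component's forward vector finds the surface it sits on.
; The physical material of that surface's first material selects Concrete, Wood, Metal or Glass audio, randomized among variants for all but concrete.
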(event Custom|Impact%20Sound
  (bind _returnvalue (Transformation|GetActorLocation))
  (bind _array (Utilities|Array|MakeArray "/Game/Sounds/Impacts/glass_impact_bullet1.glass_impact_bullet1" "/Game/Sounds/Impacts/glass_impact_bullet2.glass_impact_bullet2" "/Game/Sounds/Impacts/glass_impact_bullet3.glass_impact_bullet3" "/Game/Sounds/Impacts/glass_impact_bullet4.glass_impact_bullet4"))
  (bind _array_2 (Utilities|Array|MakeArray "/Game/Sounds/Impacts/wood_solid_impact_bullet1.wood_solid_impact_bullet1" "/Game/Sounds/Impacts/wood_solid_impact_bullet2.wood_solid_impact_bullet2" "/Game/Sounds/Impacts/wood_solid_impact_bullet3.wood_solid_impact_bullet3" "/Game/Sounds/Impacts/wood_solid_impact_bullet4.wood_solid_impact_bullet4" "/Game/Sounds/Impacts/wood_solid_impact_bullet5.wood_solid_impact_bullet5"))
  (bind _array_3 (Utilities|Array|MakeArray "/Game/Sounds/Impacts/metal_solid_impact_bullet1.metal_solid_impact_bullet1" "/Game/Sounds/Impacts/metal_solid_impact_bullet2.metal_solid_impact_bullet2" "/Game/Sounds/Impacts/metal_solid_impact_bullet3.metal_solid_impact_bullet3" "/Game/Sounds/Impacts/metal_solid_impact_bullet4.metal_solid_impact_bullet4"))
  (bind _dir (Variables|Default|Getdir))
  (bind _returnvalue_2 (Transformation|GetWorldLocation _dir))
  (bind (_outhit _returnvalue_3) (Collision|LineTraceByChannel _returnvalue_2 (+ _returnvalue_2 (* (Math|Vector|GetForwardVector (Variables|Default|Getdir)) 1.0)) "TraceTypeQuery1" false 0 "None"))
  (if _returnvalue_3
    (switch Utilities|FlowControl|Switch|SwitchonEPhysicalSurface (Variables|/Script/Engine.PhysicalMaterial|GetSurfaceType (Class|MaterialInterface|GetPhysicalMaterial (Rendering|Material|GetMaterial (.HitComponent (Collision|BreakHitResult _outhit)) 0)))
      (:SurfaceType1
        (Audio|PlaySoundatLocation "/Game/Sounds/Impacts/concrete_impact_bullet1.concrete_impact_bullet1" _returnvalue "0, 0, 0" 1.0 1.0 0.0 0 0 0))
      (:SurfaceType2
        (Audio|PlaySoundatLocation (Utilities|Array|Get(acopy) _array_2 (Math|Random|RandomIntegerinRange 0 (- (Utilities|Array|Length _array_2) 1))) _returnvalue "0, 0, 0" 1.0 1.0 0.0 0 0 0))
      (:SurfaceType3
        (Audio|PlaySoundatLocation (Utilities|Array|Get(acopy) _array_3 (Math|Random|RandomIntegerinRange 0 (- (Utilities|Array|Length _array_3) 1))) _returnvalue "0, 0, 0" 1.0 1.0 0.0 0 0 0))
      (:SurfaceType4
        (Audio|PlaySoundatLocation (Utilities|Array|Get(acopy) _array (Math|Random|RandomIntegerinRange 0 (- (Utilities|Array|Length _array) 1))) _returnvalue "0, 0, 0" 1.0 1.0 0.0 0 0 0)))))

(event EventBeginPlay
  (CallFunction|ImpactSound)
  (Utilities|FlowControl|Delay 5.0)
  (Actor|DestroyActor))

(fn ConstructionScript)