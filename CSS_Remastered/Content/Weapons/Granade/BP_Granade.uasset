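; Grenade weapon that plays pin-pull, hold and throw animations, with ammo pickup and getters for ammo count and weapon type.
; Fire pulls the pin and LetgoFire releases it, with two Tick-polled Gates and a DoOnce delaying the throw until both the pull montage finishes and release occurs.
; The throw spawns BP_Granade_THROWN with a forward impulse, spends ammo, then calls Draw to redeploy and reset the gates.
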(event EventGiveAmmo
  (params (Amount :type Integer))
  (Variables|Default|SetAmmo (+ (Variables|Default|GetAmmo) Amount))
  (Audio|PlaySoundatLocation "/Game/Sounds/ammopickup.ammopickup" (Transformation|GetActorLocation) "0, 0, 0" 1.0 1.0 0.0 0 0 0))

(event EventDraw
  (bind _granade (Variables|Default|GetGranade))
  (bind _returnvalue (Components|SkeletalMesh|GetAnimInstance _granade))
  (Variables|Default|SetCanFire false)
  (bind _returnvalue_2 (Animation|Montage|MontagePlay _returnvalue "/Game/Weapons/Granade/Models/View/Granade_Anim_v_eq_fraggrenade_qc_skeleton_deploy_Montage.Granade_Anim_v_eq_fraggrenade_qc_skeleton_deploy_Montage" 1.0 "Duration" 0.0 true))
  (Utilities|FlowControl|Delay _returnvalue_2)
  (Variables|Default|SetCanFire true)
  (Utilities|FlowControl|Sequence
    (:then_0
      (Utilities|FlowControl|Gate true) ; enters at Close
    )
    (:then_1
      (Utilities|FlowControl|Gate true) ; enters at Close
    )
    (:then_2
      (Utilities|FlowControl|DoOnce false) ; enters at Reset
    )))

(event EventFire
  (params (Camera :type Camera%20Component%20Object%20Reference))
  (bind _granade (Variables|Default|GetGranade))
  (bind _returnvalue (Components|SkeletalMesh|GetAnimInstance _granade))
  (if (and (Variables|Default|GetCanFire) (> (Variables|Default|GetAmmo) 0))
    (Variables|Default|SetCanFire false)
    (bind _returnvalue_2 (Animation|Montage|MontagePlay _returnvalue "/Game/Weapons/Granade/Models/View/Granade_Anim_v_eq_fraggrenade_qc_skeleton_pullpin_Montage.Granade_Anim_v_eq_fraggrenade_qc_skeleton_pullpin_Montage" 1.0 "MontageLength" 0.0 true))
    (bind _asgranade_abp (Utilities|Casting|CastToGranade_ABP _returnvalue))
    (Variables|/Game/Weapons/Granade/Anims/Granade_ABP.Granade_ABP_C|SetIsHolding _asgranade_abp true)
    (Utilities|FlowControl|Delay _returnvalue_2)
    (Utilities|FlowControl|Gate true) ; enters at Open
  ))

(event EventTick
  (params (DeltaSeconds :type Float%20%28single-precision%29))
  (bind _granade (Variables|Default|GetGranade))
  (bind _returnvalue (Components|SkeletalMesh|GetAnimInstance _granade))
  (Utilities|FlowControl|Sequence
    (:then_0
      (Utilities|FlowControl|Gate true
        (:Exit
          (Utilities|FlowControl|Gate true
            (:Exit
              (Utilities|FlowControl|DoOnce false
                (:Completed
                  (bind _returnvalue_2 (Animation|Montage|MontagePlay _returnvalue "/Game/Weapons/Granade/Models/View/Granade_Anim_v_eq_fraggrenade_qc_skeleton_throw_Montage.Granade_Anim_v_eq_fraggrenade_qc_skeleton_throw_Montage" 1.0 "Duration" 0.0 true))
                  (bind _returnvalue_3 (Game|SpawnActorfromClass "/Game/Weapons/Granade/BP_Granade_THROWN.BP_Granade_THROWN_C" (Transformation|GetWorldTransform (Variables|Default|GetForward)) "Undefined" self 0))
                  (Math|Integer|DecrementInt (Variables|Default|GetAmmo)
                    (:%20%20
                      (Physics|AddImpulse (Variables|/Game/Weapons/Granade/BP_Granade_THROWN.BP_Granade_THROWN_C|GetGranade_World_THROWN _returnvalue_3) (* (Math|Vector|GetForwardVector (Variables|Default|GetForward)) 2.5e+03) "None" true)
                      (bind _asgranade_abp (Utilities|Casting|CastToGranade_ABP _returnvalue))
                      (Variables|/Game/Weapons/Granade/Anims/Granade_ABP.Granade_ABP_C|SetIsHolding _asgranade_abp false)
                      (Utilities|FlowControl|Delay _returnvalue_2)
                      (CallFunction|Draw))))))))))))

(event EventLetgoFire
  (bind _granade (Variables|Default|GetGranade))
  (bind _returnvalue (Components|SkeletalMesh|GetAnimInstance _granade))
  (Utilities|FlowControl|Gate true) ; enters at Open
)

(fn ConstructionScript)

(fn DoesReplaceWeapon
  (return false))

(fn GetAmmo
  (return (Variables|Default|GetAmmo)))

(fn GetType
  (return "NewEnumerator3"))