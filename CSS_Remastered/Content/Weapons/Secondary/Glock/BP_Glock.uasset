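; Glock secondary weapon that plays draw, fire and reload montages, gating actions with CanFire and montage-length delays.
; Fire is throttled by a DoOnce and FireRate, flashes the muzzle, and line-traces from the camera to push physics objects and attach bullet holes.
; The last round auto-reloads; empty clicks use a DoOnce reset by LetgoFire.
; Drop throws a spawned pickup and destroys the weapon, while getters report ammo, type, picture and replacement behavior.
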(event EventDrop
  (params (CameraForward :type Scene%20Component%20Object%20Reference))
  (bind _returnvalue (Game|SpawnActorfromClass "/Game/Weapons/Secondary/Glock/BP_Glock_Pickup.BP_Glock_Pickup_C" (Math|Conversions|ToTransform(Vector) (Transformation|GetWorldLocation CameraForward)) "Undefined" (Components|GetOwner) 0))
  (Physics|AddForce (Variables|/Game/Weapons/Secondary/Glock/BP_Glock_Pickup.BP_Glock_Pickup_C|GetGlock_Pickup _returnvalue) (+ (* (Math|Vector|GetForwardVector CameraForward) 5e+04) (* (Math|Vector|GetUpVector CameraForward) 2.5e+04)) "None" true)
  (Actor|DestroyActor))

(event EventDraw
  (Variables|Default|SetCanFire false)
  (bind _returnvalue (Animation|Montage|MontagePlay (Components|SkeletalMesh|GetAnimInstance (Variables|Default|GetGlock)) "/Game/Weapons/Secondary/Glock/Models/View/Glock_Anim_v_pist_glock18_qc_skeleton_glock_draw_Montage.Glock_Anim_v_pist_glock18_qc_skeleton_glock_draw_Montage" 1.0 "MontageLength" 0.0 true))
  (Utilities|FlowControl|Delay _returnvalue)
  (Variables|Default|SetCanFire true))

(event EventFire
  (params (Camera :type Camera%20Component%20Object%20Reference))
  (bind _returnvalue (Transformation|GetWorldLocation Camera))
  (bind _returnvalue_2 (Math|Vector|GetForwardVector Camera))
  (bind _muzzleflash (Variables|Default|GetMuzzleFlash))
  (if (Variables|Default|GetCanFire)
    (if (> (Variables|Default|GetAmmo) 0)
      (Utilities|FlowControl|DoOnce false :!label _label
        (:Completed
          (Utilities|FlowControl|Sequence
            (:then_0
              (if (<= (Variables|Default|GetAmmo) 1)
                (bind _returnvalue_3 (Animation|Montage|MontagePlay (Components|SkeletalMesh|GetAnimInstance (Variables|Default|GetGlock)) "/Game/Weapons/Secondary/Glock/Models/View/Glock_Anim_v_pist_glock18_qc_skeleton_glock_firelast_Montage.Glock_Anim_v_pist_glock18_qc_skeleton_glock_firelast_Montage" 1.0 "MontageLength" 0.0 true))
                (Utilities|FlowControl|Sequence
                  (:then_0
                    (Utilities|FlowControl|Delay (- _returnvalue_3 0.2))
                    (CallFunction|Reload))
                  (:then_1
                    (Audio|PlaySoundatLocation "/Game/Weapons/Secondary/Glock/Sounds/glock18-1.glock18-1" (Transformation|GetActorLocation) "0, 0, 0" 1.0 1.0 0.0 0 0 0 :!label _label_2)
                    (Utilities|FlowControl|Delay (Variables|Default|GetFireRate))
                    (goto _label Reset)))
                (else
                  (Animation|Montage|MontagePlay (Components|SkeletalMesh|GetAnimInstance (Variables|Default|GetGlock)) "/Game/Weapons/Secondary/Glock/Models/View/Glock_Anim_v_pist_glock18_qc_skeleton_glock_firesingle_Montage.Glock_Anim_v_pist_glock18_qc_skeleton_glock_firesingle_Montage" 1.0 "MontageLength" 0.0 true)
                  (goto _label_2))))
            (:then_1
              (Math|Integer|DecrementInt (Variables|Default|GetAmmo)
                (:%20%20
                  (Transformation|SetRelativeRotation _muzzleflash (Math|Rotator|MakeRotator 1.8e+02 0.0 (Math|Random|RandomFloatinRange 0.0 3.6e+02)) false false)
                  (Rendering|SetVisibility _muzzleflash true false)
                  (Utilities|FlowControl|Delay 0.05)
                  (Rendering|SetVisibility _muzzleflash false false))))
            (:then_2
              (bind (_outhit _returnvalue_4) (Collision|LineTraceByChannel _returnvalue (+ _returnvalue (* _returnvalue_2 1e+04)) "TraceTypeQuery1" false 0 "None"))
              (if _returnvalue_4
                (if (Physics|IsSimulatingPhysics (.HitComponent (Collision|BreakHitResult _outhit)) "None")
                  (Physics|AddForce (.HitComponent (Collision|BreakHitResult _outhit)) (* _returnvalue_2 6e+04) "None" true))
                (bind _returnvalue_5 (Game|SpawnActorfromClass "/Game/Objects/Bullethole/BP_Bullethole.BP_Bullethole_C" (Math|Transform|MakeTransform (.Location (Collision|BreakHitResult _outhit)) (Math|Rotator|MakeRotfromZ (.Normal (Collision|BreakHitResult _outhit)))) "Undefined" 0 0))
                (Transformation|AttachComponentToComponent _returnvalue_5 (.HitComponent (Collision|BreakHitResult _outhit)) "None" "KeepWorld" "KeepWorld" "KeepWorld" true))))))
      (else
        (Utilities|FlowControl|DoOnce false
          (:Completed
            (Audio|PlaySoundatLocation "/Game/Weapons/Secondary/USP/Sounds/clipempty_pistol.clipempty_pistol" (Transformation|GetActorLocation) "0, 0, 0" 1.0 1.0 0.0 0 0 0)))))))

(event EventLetgoFire
  (Utilities|FlowControl|DoOnce false) ; enters at Reset
)

(event EventReload
  (if (and (Variables|Default|GetCanFire) (< (Variables|Default|GetAmmo) (Variables|Default|GetMaxAmmo)))
    (Variables|Default|SetCanFire false)
    (bind _returnvalue (Animation|Montage|MontagePlay (Components|SkeletalMesh|GetAnimInstance (Variables|Default|GetGlock)) "/Game/Weapons/Secondary/Glock/Models/View/Glock_Anim_v_pist_glock18_qc_skeleton_glock_reload_Montage.Glock_Anim_v_pist_glock18_qc_skeleton_glock_reload_Montage" 1.0 "MontageLength" 0.0 true))
    (Utilities|FlowControl|Delay (- _returnvalue 0.7))
    (Variables|Default|SetAmmo (Variables|Default|GetMaxAmmo))
    (Variables|Default|SetCanFire true)))

(fn ConstructionScript
  (Variables|Default|SetAmmo (Variables|Default|GetMaxAmmo)))

(fn DoesReplaceWeapon
  (return true))

(fn GetAmmo
  (return (Variables|Default|GetAmmo)))

(fn GetType
  (return "NewEnumerator1"))

(fn GetWeaponPic
  (return "/Game/Weapons/Secondary/Glock/Textures/glock18.glock18"))