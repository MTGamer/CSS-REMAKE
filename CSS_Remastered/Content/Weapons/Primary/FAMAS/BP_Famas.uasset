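; First-person FAMAS primary weapon with automatic fire, ammo, draw and reload montages, and queries for ammo, type and HUD picture.
; Fire and LetgoFire open and close a Tick gate, with a delayed DoOnce pacing shots.
; Each shot line-traces from the saved camera, pushes physics bodies, attaches a bullet hole and flashes the muzzle.
; Drop spawns and throws a BP_Famas_World pickup, then destroys this actor.
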(event EventDrop
  (params (CameraForward :type Scene%20Component%20Object%20Reference))
  (bind _returnvalue (Game|SpawnActorfromClass "/Game/Weapons/Primary/FAMAS/BP_Famas_World.BP_Famas_World_C" (Math|Conversions|ToTransform(Vector) (Transformation|GetWorldLocation CameraForward)) "Undefined" (Components|GetOwner) 0))
  (Physics|AddForce (Variables|/Game/Weapons/Primary/FAMAS/BP_Famas_World.BP_Famas_World_C|GetFamas_World _returnvalue) (+ (* (Math|Vector|GetForwardVector CameraForward) 5e+04) (* (Math|Vector|GetUpVector CameraForward) 2.5e+04)) "None" true)
  (Actor|DestroyActor))

(event EventDraw
  (Variables|Default|SetCanFire false)
  (bind _returnvalue (Animation|Montage|MontagePlay (Components|SkeletalMesh|GetAnimInstance (Variables|Default|GetFamas)) "/Game/Weapons/Primary/FAMAS/Models/View/Famas_Anim_v_rif_famas_qc_skeleton_draw_Montage.Famas_Anim_v_rif_famas_qc_skeleton_draw_Montage" 1.0 "MontageLength" 0.0 true))
  (Utilities|FlowControl|Delay _returnvalue)
  (Variables|Default|SetCanFire true))

(event EventFire
  (params (Camera :type Camera%20Component%20Object%20Reference))
  (bind _muzzleflash (Variables|Default|GetMuzzleFlash))
  (Variables|Default|SetSavedCam Camera)
  (Utilities|FlowControl|Gate true) ; enters at Open
)

(event EventLetgoFire
  (bind _muzzleflash (Variables|Default|GetMuzzleFlash))
  (Utilities|FlowControl|Sequence
    (:then_0
      (Variables|Default|SetSavedCam 0)
      (Utilities|FlowControl|Gate true) ; enters at Close
    )
    (:then_1
      (Utilities|FlowControl|DoOnce false) ; enters at Reset
    )))

(event EventTick
  (params (DeltaSeconds :type Float%20%28single-precision%29))
  (bind _muzzleflash (Variables|Default|GetMuzzleFlash))
  (bind _savedcam (Variables|Default|GetSavedCam))
  (bind _returnvalue (Transformation|GetWorldLocation _savedcam))
  (bind _returnvalue_2 (Math|Vector|GetForwardVector _savedcam))
  (Utilities|FlowControl|Gate true
    (:Exit
      (if (Variables|Default|GetCanFire)
        (if (> (Variables|Default|GetAmmo) 0)
          (Utilities|FlowControl|DoOnce false :!label _label
            (:Completed
              (Utilities|FlowControl|Sequence
                (:then_0
                  (Animation|Montage|MontagePlay (Components|SkeletalMesh|GetAnimInstance (Variables|Default|GetFamas)) "/Game/Weapons/Primary/FAMAS/Models/View/Famas_Anim_v_rif_famas_qc_skeleton_shoot1_Montage.Famas_Anim_v_rif_famas_qc_skeleton_shoot1_Montage" 1.0 "MontageLength" 0.0 true)
                  (Audio|PlaySoundatLocation "/Game/Weapons/Primary/FAMAS/Sounds/famas-1.famas-1" (Transformation|GetActorLocation) "0, 0, 0" 1.0 1.0 0.0 0 0 0)
                  (Utilities|FlowControl|Delay (Variables|Default|GetFireRate))
                  (goto _label Reset))
                (:then_1
                  (Math|Integer|DecrementInt (Variables|Default|GetAmmo)
                    (:%20%20
                      (bind (_outhit _returnvalue_3) (Collision|LineTraceByChannel _returnvalue (+ (* _returnvalue_2 1e+04) _returnvalue) "TraceTypeQuery1" false 0 "None"))
                      (if _returnvalue_3
                        (if (Physics|IsSimulatingPhysics (.HitComponent (Collision|BreakHitResult _outhit)) "None")
                          (Physics|AddForce (.HitComponent (Collision|BreakHitResult _outhit)) (* _returnvalue_2 6e+04) "None" true))
                        (bind _returnvalue_4 (Game|SpawnActorfromClass "/Game/Objects/Bullethole/BP_Bullethole.BP_Bullethole_C" (Math|Transform|MakeTransform (.Location (Collision|BreakHitResult _outhit)) (Math|Rotator|MakeRotfromZ (.Normal (Collision|BreakHitResult _outhit)))) "Undefined" 0 0))
                        (Transformation|AttachComponentToComponent _returnvalue_4 (.HitComponent (Collision|BreakHitResult _outhit)) "None" "KeepWorld" "KeepWorld" "KeepWorld" true)))))
                (:then_2
                  (Transformation|SetRelativeRotation _muzzleflash (Math|Rotator|MakeRotator 1.8e+02 0.0 (Math|Random|RandomFloatinRange 0.0 3.6e+02)) false false)
                  (Rendering|SetVisibility _muzzleflash true false)
                  (Utilities|FlowControl|Delay 0.05)
                  (Rendering|SetVisibility _muzzleflash false false)))))
          (else
            (Utilities|FlowControl|DoOnce false
              (:Completed
                (Audio|PlaySoundatLocation "/Game/Weapons/Primary/AK47/Sounds/clipempty_rifle.clipempty_rifle" (Transformation|GetActorLocation) "0, 0, 0" 1.0 1.0 0.0 0 0 0)))))))))

(event EventReload
  (if (and (Variables|Default|GetCanFire) (< (Variables|Default|GetAmmo) (Variables|Default|GetMaxAmmo)))
    (Variables|Default|SetCanFire false)
    (bind _returnvalue (Animation|Montage|MontagePlay (Components|SkeletalMesh|GetAnimInstance (Variables|Default|GetFamas)) "/Game/Weapons/Primary/FAMAS/Models/View/Famas_Anim_v_rif_famas_qc_skeleton_reload_Montage.Famas_Anim_v_rif_famas_qc_skeleton_reload_Montage" 1.0 "MontageLength" 0.0 true))
    (Utilities|FlowControl|Delay _returnvalue)
    (Variables|Default|SetAmmo (Variables|Default|GetMaxAmmo))
    (Variables|Default|SetCanFire true)))

(fn ConstructionScript
  (Variables|Default|SetAmmo (Variables|Default|GetMaxAmmo)))

(fn DoesReplaceWeapon
  (return true))

(fn GetAmmo
  (return (Variables|Default|GetAmmo)))

(fn GetType
  (return "NewEnumerator0"))

(fn GetWeaponPic
  (return "/Game/Weapons/Primary/FAMAS/Textures/famas.famas"))