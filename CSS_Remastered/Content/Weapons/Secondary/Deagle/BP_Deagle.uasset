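; Deagle secondary weapon actor that handles drawing, firing, reloading and dropping, and exposes ammo, type and picture through getters.
; Fire runs a camera line trace that pushes physics objects and attaches bullet holes, with sound, animation and a brief randomly rotated muzzle flash.
; DoOnce and delays pace firing and reloading, montage lengths time draw and reload, and an empty magazine auto-reloads.
; Drop spawns a thrown pickup and destroys the weapon.
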(event EventDrop
  (params (CameraForward :type Scene%20Component%20Object%20Reference))
  (bind _returnvalue (Game|SpawnActorfromClass "/Game/Weapons/Secondary/Deagle/BP_Deagle_Pickup.BP_Deagle_Pickup_C" (Math|Conversions|ToTransform(Vector) (Transformation|GetWorldLocation CameraForward)) "Undefined" (Components|GetOwner) 0))
  (Physics|AddForce (Variables|/Game/Weapons/Secondary/Deagle/BP_Deagle_Pickup.BP_Deagle_Pickup_C|GetDeagle_Pickup _returnvalue) (+ (* (Math|Vector|GetForwardVector CameraForward) 5e+04) (* (Math|Vector|GetUpVector CameraForward) 2.5e+04)) "None" true)
  (Actor|DestroyActor))

(event EventDraw
  (Variables|Default|SetCanFire false)
  (bind _returnvalue (Animation|Montage|MontagePlay (Components|SkeletalMesh|GetAnimInstance (Variables|Default|GetDeagle)) "/Game/Weapons/Secondary/Deagle/Models/View/Deagle_Anim_v_pist_deagle_qc_skeleton_draw_Montage.Deagle_Anim_v_pist_deagle_qc_skeleton_draw_Montage" 1.0 "MontageLength" 0.0 true))
  (Utilities|FlowControl|Delay _returnvalue)
  (Variables|Default|SetCanFire true))

(event EventFire
  (params (Camera :type Camera%20Component%20Object%20Reference))
  (bind _returnvalue (Math|Vector|GetForwardVector Camera))
  (bind _returnvalue_2 (Transformation|GetWorldLocation Camera))
  (bind _deagle (Variables|Default|GetDeagle))
  (bind _muzzleflash (Variables|Default|GetMuzzleFlash))
  (bind _firerate (Variables|Default|GetFireRate))
  (bind _returnvalue_3 (Components|SkeletalMesh|GetAnimInstance _deagle))
  (if (and (> (Variables|Default|GetAmmo) 0) (Variables|Default|GetCanFire))
    (Utilities|FlowControl|DoOnce false :!label _label
      (:Completed
        (Utilities|FlowControl|Sequence
          (:then_0
            (Math|Integer|DecrementInt (Variables|Default|GetAmmo)
              (:%20%20
                (bind (_outhit _returnvalue_4) (Collision|LineTraceByChannel _returnvalue_2 (+ _returnvalue_2 (* _returnvalue 1e+04)) "TraceTypeQuery1" false 0 "None"))
                (if _returnvalue_4
                  (if (Physics|IsSimulatingPhysics (.HitComponent (Collision|BreakHitResult _outhit)) "None")
                    (Physics|AddForce (.HitComponent (Collision|BreakHitResult _outhit)) (* _returnvalue 3e+04) "None" true))
                  (bind _returnvalue_5 (Game|SpawnActorfromClass "/Game/Objects/Bullethole/BP_Bullethole.BP_Bullethole_C" (Math|Transform|MakeTransform (.Location (Collision|BreakHitResult _outhit)) (Math|Rotator|MakeRotfromZ (.Normal (Collision|BreakHitResult _outhit)))) "Undefined" 0 0))
                  (Transformation|AttachComponentToComponent _returnvalue_5 (.HitComponent (Collision|BreakHitResult _outhit)) "None" "KeepWorld" "KeepWorld" "KeepWorld" true)))))
          (:then_1
            (Audio|PlaySoundatLocation "/Game/Weapons/Secondary/Deagle/Sounds/deagle-1.deagle-1" (Transformation|GetActorLocation) "0, 0, 0" 1.0 1.0 0.0 0 0 0)
            (if (<= (Variables|Default|GetAmmo) 0)
              (bind _returnvalue_6 (Animation|Montage|MontagePlay _returnvalue_3 "/Game/Weapons/Secondary/Deagle/Models/View/Deagle_Anim_v_pist_deagle_qc_skeleton_shoot_empty_Montage.Deagle_Anim_v_pist_deagle_qc_skeleton_shoot_empty_Montage" 1.0 "MontageLength" 0.0 true))
              (Utilities|FlowControl|Sequence
                (:then_0
                  (Utilities|FlowControl|Delay _firerate)
                  (goto _label Reset))
                (:then_1
                  (Utilities|FlowControl|Delay (- _returnvalue_6 0.2))
                  (CallFunction|Reload)))
              (else
                (Animation|Montage|MontagePlay _returnvalue_3 "/Game/Weapons/Secondary/Deagle/Models/View/Deagle_Anim_v_pist_deagle_qc_skeleton_shoot1_Montage.Deagle_Anim_v_pist_deagle_qc_skeleton_shoot1_Montage" 1.0 "MontageLength" 0.0 true)
                (Utilities|FlowControl|Delay _firerate)
                (goto _label Reset))))
          (:then_2
            (Transformation|SetRelativeRotation _muzzleflash (Math|Rotator|MakeRotator -90.000137 (Math|Random|RandomFloatinRange 0.0 3.6e+02) 0.0) false false)
            (Rendering|SetVisibility _muzzleflash true false)
            (Utilities|FlowControl|Delay 0.05)
            (Rendering|SetVisibility _muzzleflash false false)))))))

(event EventReload
  (if (< (Variables|Default|GetAmmo) (Variables|Default|GetMaxAmmo))
    (Utilities|FlowControl|DoOnce false :!label _label
      (:Completed
        (Variables|Default|SetCanFire false)
        (bind _returnvalue (Animation|Montage|MontagePlay (Components|SkeletalMesh|GetAnimInstance (Variables|Default|GetDeagle)) "/Game/Weapons/Secondary/Deagle/Models/View/Deagle_Anim_v_pist_deagle_qc_skeleton_reload_Montage.Deagle_Anim_v_pist_deagle_qc_skeleton_reload_Montage" 1.0 "MontageLength" 0.0 true))
        (Utilities|FlowControl|Delay _returnvalue)
        (Variables|Default|SetCanFire true)
        (Variables|Default|SetAmmo (Variables|Default|GetMaxAmmo))
        (goto _label Reset)))))

(fn ConstructionScript
  (Variables|Default|SetAmmo (Variables|Default|GetMaxAmmo)))

(fn DoesReplaceWeapon
  (return true))

(fn GetAmmo
  (return (Variables|Default|GetAmmo)))

(fn GetType
  (return (Variables|Default|GetType)))

(fn GetWeaponPic
  (return "/Game/Weapons/Secondary/Deagle/Textures/deserteagle.deserteagle"))