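; M4A1 weapon Blueprint: an automatic hitscan rifle with a detachable silencer, ammo, reload, draw and drop-as-pickup.
; Fire and LetgoFire toggle a Tick-driven gate, with a delayed DoOnce setting fire rate.
; Shots trace from the passed camera, pushing physics objects and attaching bullet holes, without applying damage.
; HasSil feeds the AnimBP and selects montages, shot sounds and muzzle flash, while CanFire locks actions during draw, reload and silencer swaps.
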(event EventAlt
  (params (Camera :type Camera%20Component%20Object%20Reference))
  (bind _m4a1 (Variables|Default|GetM4A1))
  (bind _returnvalue (Components|SkeletalMesh|GetAnimInstance _m4a1))
  (if (Variables|Default|GetCanFire)
    (Variables|Default|SetCanFire false)
    (if (Variables|Default|GetHasSil)
      (bind _returnvalue_2 (Animation|Montage|MontagePlay _returnvalue "/Game/Weapons/Primary/M4A1/Models/View/M4A1_Anim_v_rif_m4a1_qc_skeleton_detach_silencer_Montage.M4A1_Anim_v_rif_m4a1_qc_skeleton_detach_silencer_Montage" 1.0 "MontageLength" 0.0 true))
      (Utilities|FlowControl|Sequence
        (:then_0
          (Utilities|FlowControl|Delay _returnvalue_2)
          (Variables|Default|SetCanFire true :!label _label))
        (:then_1
          (Utilities|FlowControl|Delay (- _returnvalue_2 1.2))
          (Variables|Default|SetHasSil (not (Variables|Default|GetHasSil)) :!label _label_2)))
      (else
        (bind _returnvalue_3 (Animation|Montage|MontagePlay _returnvalue "/Game/Weapons/Primary/M4A1/Models/View/M4A1_Anim_v_rif_m4a1_qc_skeleton_add_silencer_Montage.M4A1_Anim_v_rif_m4a1_qc_skeleton_add_silencer_Montage" 1.0 "MontageLength" 0.0 true))
        (Utilities|FlowControl|Sequence
          (:then_0
            (Utilities|FlowControl|Delay _returnvalue_3)
            (goto _label))
          (:then_1
            (Utilities|FlowControl|Delay (- _returnvalue_3 0.5))
            (goto _label_2)))))))

(event EventDrop
  (params (CameraForward :type Scene%20Component%20Object%20Reference))
  (bind _returnvalue (Game|SpawnActorfromClass "/Game/Weapons/Primary/M4A1/BP_M4A1_Pickup.BP_M4A1_Pickup_C" (Math|Conversions|ToTransform(Vector) (Transformation|GetWorldLocation CameraForward)) "Undefined" (Components|GetOwner) 0))
  (Physics|AddForce (Variables|/Game/Weapons/Primary/M4A1/BP_M4A1_Pickup.BP_M4A1_Pickup_C|GetM4A1_Pickup _returnvalue) (+ (* (Math|Vector|GetForwardVector CameraForward) 5e+04) (* (Math|Vector|GetUpVector CameraForward) 2.5e+04)) "None" true)
  (Actor|DestroyActor))

(event EventFire
  (params (Camera :type Camera%20Component%20Object%20Reference))
  (bind _returnvalue (Transformation|GetActorLocation))
  (bind _muzzlefash (Variables|Default|GetMuzzleFash))
  (bind _ammo (Variables|Default|GetAmmo))
  (bind _m4a1 (Variables|Default|GetM4A1))
  (bind _returnvalue_2 (Components|SkeletalMesh|GetAnimInstance _m4a1))
  (Variables|Default|SetCamera Camera)
  (Utilities|FlowControl|Gate true) ; enters at Open
)

(event EventDraw
  (bind _m4a1 (Variables|Default|GetM4A1))
  (bind _returnvalue (Components|SkeletalMesh|GetAnimInstance _m4a1))
  (Variables|Default|SetCanFire false)
  (if (Variables|Default|GetHasSil)
    (bind _returnvalue_2 (Animation|Montage|MontagePlay _returnvalue "/Game/Weapons/Primary/M4A1/Models/View/M4A1_Anim_v_rif_m4a1_qc_skeleton_draw_Montage.M4A1_Anim_v_rif_m4a1_qc_skeleton_draw_Montage" 1.0 "MontageLength" 0.0 true))
    (Utilities|FlowControl|Delay _returnvalue_2)
    (else
      (bind _returnvalue_3 (Animation|Montage|MontagePlay _returnvalue "/Game/Weapons/Primary/M4A1/Models/View/M4A1_Anim_v_rif_m4a1_qc_skeleton_draw_unsil_Montage.M4A1_Anim_v_rif_m4a1_qc_skeleton_draw_unsil_Montage" 1.0 "MontageLength" 0.0 true))
      (Utilities|FlowControl|Delay _returnvalue_3)))
  (Variables|Default|SetCanFire true))

(event EventLetgoFire
  (bind _returnvalue (Transformation|GetActorLocation))
  (bind _muzzlefash (Variables|Default|GetMuzzleFash))
  (bind _ammo (Variables|Default|GetAmmo))
  (bind _m4a1 (Variables|Default|GetM4A1))
  (bind _returnvalue_2 (Components|SkeletalMesh|GetAnimInstance _m4a1))
  (Utilities|FlowControl|Sequence
    (:then_0
      (Variables|Default|SetCamera 0)
      (Utilities|FlowControl|Gate true) ; enters at Close
    )
    (:then_1
      (Utilities|FlowControl|DoOnce false) ; enters at Reset
    )))

(event EventReload
  (bind _m4a1 (Variables|Default|GetM4A1))
  (bind _returnvalue (Components|SkeletalMesh|GetAnimInstance _m4a1))
  (if (and (Variables|Default|GetCanFire) (< (Variables|Default|GetAmmo) (Variables|Default|GetMaxAmmo)))
    (Variables|Default|SetCanFire false)
    (if (Variables|Default|GetHasSil)
      (bind _returnvalue_2 (Animation|Montage|MontagePlay _returnvalue "/Game/Weapons/Primary/M4A1/Models/View/M4A1_Anim_v_rif_m4a1_qc_skeleton_reload_Montage.M4A1_Anim_v_rif_m4a1_qc_skeleton_reload_Montage" 1.0 "MontageLength" 0.0 true))
      (Utilities|FlowControl|Delay _returnvalue_2)
      (else
        (bind _returnvalue_3 (Animation|Montage|MontagePlay _returnvalue "/Game/Weapons/Primary/M4A1/Models/View/M4A1_Anim_v_rif_m4a1_qc_skeleton_reload_unsil_Montage.M4A1_Anim_v_rif_m4a1_qc_skeleton_reload_unsil_Montage" 1.0 "MontageLength" 0.0 true))
        (Utilities|FlowControl|Delay _returnvalue_3)))
    (Variables|Default|SetAmmo (Variables|Default|GetMaxAmmo))
    (Variables|Default|SetCanFire true)))

(event EventTick
  (params (DeltaSeconds :type Float%20%28single-precision%29))
  (bind _returnvalue (Transformation|GetActorLocation))
  (bind _muzzlefash (Variables|Default|GetMuzzleFash))
  (bind _ammo (Variables|Default|GetAmmo))
  (bind _m4a1 (Variables|Default|GetM4A1))
  (bind _camera (Variables|Default|GetCamera))
  (bind _returnvalue_2 (Transformation|GetWorldLocation _camera))
  (bind _returnvalue_3 (Math|Vector|GetForwardVector _camera))
  (bind _returnvalue_4 (Components|SkeletalMesh|GetAnimInstance _m4a1))
  (Utilities|FlowControl|Sequence
    (:then_0
      (bind _asm4a1_abp (Utilities|Casting|CastToM4A1_ABP (Components|SkeletalMesh|GetAnimInstance (Variables|Default|GetM4A1))))
      (Variables|/Game/Weapons/Primary/M4A1/Anims/M4A1_ABP.M4A1_ABP_C|SetHasSil _asm4a1_abp (Variables|Default|GetHasSil)))
    (:then_1
      (Utilities|FlowControl|Gate true
        (:Exit
          (if (Variables|Default|GetCanFire)
            (if (> (Variables|Default|GetAmmo) 0)
              (Utilities|FlowControl|DoOnce false :!label _label
                (:Completed
                  (Utilities|FlowControl|Sequence
                    (:then_0
                      (if (Variables|Default|GetHasSil)
                        (Math|Integer|DecrementInt _ammo
                          (:%20%20
                            (Audio|PlaySoundatLocation "/Game/Weapons/Primary/M4A1/Sounds/m4a1-1.m4a1-1" _returnvalue "0, 0, 0" 1.0 1.0 0.0 0 0 0)
                            (Animation|Montage|MontagePlay _returnvalue_4 "/Game/Weapons/Primary/M4A1/Models/View/M4A1_Anim_v_rif_m4a1_qc_skeleton_shoot1_Montage.M4A1_Anim_v_rif_m4a1_qc_skeleton_shoot1_Montage" 1.0 "MontageLength" 0.0 true)))
                        (else
                          (Math|Integer|DecrementInt _ammo
                            (:%20%20
                              (Audio|PlaySoundatLocation "/Game/Weapons/Primary/M4A1/Sounds/m4a1_unsil-1.m4a1_unsil-1" _returnvalue "0, 0, 0" 1.0 1.0 0.0 0 0 0)
                              (Animation|Montage|MontagePlay _returnvalue_4 "/Game/Weapons/Primary/M4A1/Models/View/M4A1_Anim_v_rif_m4a1_qc_skeleton_shoot1_unsil_Montage.M4A1_Anim_v_rif_m4a1_qc_skeleton_shoot1_unsil_Montage" 1.0 "MontageLength" 0.0 true)))))
                      (Utilities|FlowControl|Delay (Variables|Default|GetFireRate))
                      (goto _label Reset))
                    (:then_1
                      (bind (_outhit _returnvalue_5) (Collision|LineTraceByChannel _returnvalue_2 (+ (* _returnvalue_3 1e+04) _returnvalue_2) "TraceTypeQuery1" false 0 "None"))
                      (if _returnvalue_5
                        (if (Physics|IsSimulatingPhysics (.HitComponent (Collision|BreakHitResult _outhit)) "None")
                          (Physics|AddForce (.HitComponent (Collision|BreakHitResult _outhit)) (* _returnvalue_3 6e+04) "None" true))
                        (bind _returnvalue_6 (Game|SpawnActorfromClass "/Game/Objects/Bullethole/BP_Bullethole.BP_Bullethole_C" (Math|Transform|MakeTransform (.Location (Collision|BreakHitResult _outhit)) (Math|Rotator|MakeRotfromZ (.Normal (Collision|BreakHitResult _outhit)))) "Undefined" 0 0))
                        (Transformation|AttachComponentToComponent _returnvalue_6 (.HitComponent (Collision|BreakHitResult _outhit)) "None" "KeepWorld" "KeepWorld" "KeepWorld" true)))
                    (:then_2
                      (if (not (Variables|Default|GetHasSil))
                        (Transformation|SetRelativeRotation _muzzlefash (Math|Rotator|MakeRotator -1.8e+02 0.0 (Math|Random|RandomFloatinRange 0.0 3.6e+02)) false false)
                        (Rendering|SetVisibility _muzzlefash true false)
                        (Utilities|FlowControl|Delay 0.05)
                        (Rendering|SetVisibility _muzzlefash false false))))))
              (else
                (Utilities|FlowControl|DoOnce false
                  (:Completed
                    (Audio|PlaySoundatLocation "/Game/Weapons/Primary/AK47/Sounds/clipempty_rifle.clipempty_rifle" (Transformation|GetActorLocation) "0, 0, 0" 1.0 1.0 0.0 0 0 0)))))))))))

(fn ConstructionScript
  (Variables|Default|SetAmmo (Variables|Default|GetMaxAmmo)))

(fn DoesReplaceWeapon
  (return true))

(fn GetAmmo
  (return (Variables|Default|GetAmmo)))

(fn GetType
  (return "NewEnumerator0"))

(fn GetWeaponPic
  (return "/Game/Weapons/Primary/M4A1/Textures/m4a1.m4a1"))